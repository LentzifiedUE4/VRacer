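; VR racing vehicle pawn Blueprint that drives the cockpit displays and thruster-style flame effects.
; Each tick it updates pedal bars, a zero-padded speedometer, the race timer, and curve-driven flame material and light colors from tweened acceleration.
; A full left-trigger pull recenters the camera root using the hand controllers' midpoint and wheel anchor.
; Checkpoint crossings briefly freeze and flash the timer, and race resets restart the start-block lights.
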(event Custom|ShowCheckpointTime
  (bind _timerwidget (Variables|Default|GetTimerWidget))
  ;[1 1 1] Flash Checkpoint Time On Checkpoint/Start Block Crossed
  (Variables|Default|SetUpdateTimer false)
  (UserInterface|Animation|PlayAnimation _timerwidget (Variables|/Game/Widgets/TimerGui.TimerGui_C|GetLapFlash _timerwidget) 0.0 1 "Forward" 1.0 false)
  (Utilities|FlowControl|Delay 1.0)
  (Variables|Default|SetUpdateTimer true))

(event Custom|ResetRace
  ;[1 1 1] Bind And Cast Reset Race Delegate
  (bind _returnvalue (Actor|GetActorOfClass "/Game/Blueprints/StartBlock_BP.StartBlock_BP_C"))
  (Default|StartLights _returnvalue))

(event EventBeginPlay
  ;[1 1 1] Promote User Widget Objects to Variables
  (bind _asdashboard_gui (Utilities|Casting|CastToDashboardGUI (UserInterface|GetUserWidgetObject (Variables|Default|GetDashboardGui))))
  (Variables|Default|SetDashboardWidget _asdashboard_gui)
  (bind _astimer_gui (Utilities|Casting|CastToTimerGui (UserInterface|GetUserWidgetObject (Variables|Default|GetTimerGui))))
  (Variables|Default|SetTimerWidget _astimer_gui)
  ;[1 1 1] Bind And Cast Reset Race Delegate
  (EventDispatchers|BindEventtoResetRaceDelegate (delegate Custom|ResetRace)))

(event EventTick
  (params (DeltaSeconds :type Float%20%28single-precision%29))
  ;[1 1 1] Call Tick-Bound Functions
  (CallFunction|SetFlameColor)
  (CallFunction|SetDashboardBars)
  (CallFunction|SetTimerGuiText)
  (CallFunction|SetSpeedometerText))

(event Input|AxisEvents|InputAxisLeftTrigger
  (params (AxisValue :type Float%20%28single-precision%29))
  ;[1 1 1] Call Cockpit Calibration Function
  (if (== AxisValue 1.0)
    (CallFunction|CenterCharactertoWheel)))

(fn ConstructionScript
  (bind _vehiclecomponent (Variables|Default|GetVehicleComponent))
  ;[1 1 1] Define Flame Material Instance
  (bind _returnvalue (Rendering|Material|CreateDynamicMaterialInstance _vehiclecomponent 6 (Rendering|Material|GetMaterial _vehiclecomponent 6) "None" :!class /Script/Engine.PrimitiveComponent))
  (Variables|Default|SetFlameMaterial _returnvalue))

(fn CenterCharactertoWheel
  ;[1 1 1] Center Controller Median Point to Steering Wheel
  (Transformation|SetRelativeLocation (Variables|Default|GetCameraRoot) (+ (/ (+ (Variables|/Script/Engine.SceneComponent|GetRelativeLocation (Variables|Default|GetRightHand)) (Variables|/Script/Engine.SceneComponent|GetRelativeLocation (Variables|Default|GetLeftHand))) -2.0) (Variables|/Script/Engine.SceneComponent|GetRelativeLocation (Variables|Default|GetWheelAnchor))) false false))

(fn SetFlameColor
  (bind _flamecurve (Variables|Default|GetFlameCurve))
  (bind _tweenedaccel (Variables|Default|GetTweenedAccel))
  (bind _returnvalue (Math|Curves|GetLinearColorValue _flamecurve _tweenedaccel))
  ;[1 1 1] Set Flame Material and Light Colors by Vector Curve
  (Rendering|Material|SetVectorParameterValue (Variables|Default|GetFlameMaterial) "Color" (Utilities|Struct|MakeLinearColor (.r _returnvalue) (.g _returnvalue) (.b _returnvalue) (+ (* _tweenedaccel 3e+01) 15.0)) :!class /Script/Engine.MaterialInstanceDynamic)
  (Rendering|Components|Light|SetLightColor (Variables|Default|GetLightBR) (Math|Curves|GetLinearColorValue (Variables|Default|GetFlameCurve) (Variables|Default|GetTweenedAccel)) true))

(fn SetDashboardBars
  ;[1 1 1] Set Acceleration and Brake Bar Percentage on Dashboard
  (Progress|SetPercent (Variables|/Game/Widgets/DashboardGUI.DashboardGUI_C|GetAcceleratorBar (Variables|Default|GetDashboardWidget)) (Variables|Default|GetAccelInput))
  (Progress|SetPercent (Variables|/Game/Widgets/DashboardGUI.DashboardGUI_C|GetBrakesBar (Variables|Default|GetDashboardWidget)) (* (Variables|Default|GetBrakeInput) 2.0)))

(fn SetTimerGuiText
  (bind _racetime (Variables|Default|GetRaceTime))
  (bind _racetime_2 (Variables|Default|GetRaceTime))
  (bind _returnvalue (Math|Float|Floor _racetime_2))
  (bind _returnvalue_2 (* _racetime 1e+02))
  (bind _returnvalue_3 (Math|Integer|%(Integer) _returnvalue 60))
  (bind _returnvalue_4 (Math|Float|Floor _returnvalue_2))
  (bind _returnvalue_5 (Utilities|String|ToString(Integer) _returnvalue_3))
  (bind _returnvalue_6 (Math|Integer|%(Integer) _returnvalue_4 100))
  (bind _returnvalue_7 (Utilities|String|ToString(Integer) _returnvalue_6))
  ;[1 1 1] Set Steering Wheel Timer Text
  (if (Variables|Default|GetUpdateTimer)
    (Rendering|Components|TextRender|SetText (Variables|/Game/Widgets/TimerGui.TimerGui_C|GetTimerText (Variables|Default|GetTimerWidget)) (Utilities|Text|ToText(String) (Utilities|String|Append (Utilities|String|ToString(Integer) (Math|Float|Floor (/ (Variables|Default|GetRaceTime) 6e+01))) ":" (Utilities|String|SelectString (Utilities|String|Append "0" _returnvalue_5) _returnvalue_5 (< _returnvalue_3 10)) "." (Utilities|String|SelectString (Utilities|String|Append "0" _returnvalue_7) _returnvalue_7 (< _returnvalue_6 10)))))))

(fn SetSpeedometerText
  (bind _dashboardwidget (Variables|Default|GetDashboardWidget))
  (bind _speedtext (Variables|/Game/Widgets/DashboardGUI.DashboardGUI_C|GetSpeedText _dashboardwidget))
  ;[1 1 1] Set Speedometer Text in Kilometers per Hour
  ;;[1 1 1] Get Speed in KM/H
  (bind _returnvalue (Physics|GetPhysicsLinearVelocity (Variables|Default|GetVehicleComponent) "None"))
  ;;[1 1 1] Set Speed Text and Color
  (Rendering|Components|TextRender|SetText _speedtext (Utilities|Text|ToText(String) (Utilities|String|SelectString (Utilities|String|Append "00" (Utilities|String|ToString(Integer) (Math|Float|Truncate (/ (Math|Vector|VectorLength _returnvalue) 1e+02)))) (Utilities|String|SelectString (Utilities|String|Append "0" (Utilities|String|ToString(Integer) (Math|Float|Truncate (/ (Math|Vector|VectorLength _returnvalue) 1e+02)))) (Utilities|String|ToString(Integer) (Math|Float|Truncate (/ (Math|Vector|VectorLength _returnvalue) 1e+02))) (< (Math|Float|Truncate (/ (Math|Vector|VectorLength _returnvalue) 1e+02)) 100)) (< (Math|Float|Truncate (/ (Math|Vector|VectorLength _returnvalue) 1e+02)) 10))))
  (if (>= (Math|Float|Truncate (/ (Math|Vector|VectorLength _returnvalue) 1e+02)) 115)
    (Appearance|SetColorandOpacity _speedtext (Utilities|Struct|MakeSlateColor "(R=1.000000,G=0.000000,B=0.000000,A=1.000000)" "UseColor_Specified") :!class /Script/UMG.TextBlock)
    (else
      (Appearance|SetColorandOpacity _speedtext (Utilities|Struct|MakeSlateColor "(R=1.000000,G=1.000000,B=1.000000,A=1.000000)" "UseColor_Specified") :!class /Script/UMG.TextBlock))))