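; StartBlock_BP is the start/finish road block of a racing game, running the start-light countdown and registering laps.
; After a delay on BeginPlay, it cycles emissive red, yellow and green through dynamic material instances built in the Construction Script, then enables driving on every VehiclePawn_BP.
; Vehicles entering the StartOverlap trigger increment their lap count, store a checkpoint transform, show their time and restart race timing.
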(event OnComponentBeginOverlap(StartOverlap)
  (params (OverlappedComponent :type Primitive%20Component%20Object%20Reference) (OtherActor :type Actor%20Object%20Reference) (OtherComp :type Primitive%20Component%20Object%20Reference) (OtherBodyIndex :type Integer) (bFromSweep :type Boolean) (SweepResult :type Hit%20Result%20Structure%20%28by%20ref%29))
  ;[1 1 1] Modify Vehicle Race Variables on Start Box Overlapped by Vehicle
  (bind _asvehicle_pawn_bp (Utilities|Casting|CastToVehiclePawn_BP OtherActor))
  (Math|Integer|IncrementInt (Variables|/Script/VRacer.VehiclePawn|GetLapCount _asvehicle_pawn_bp)
    (:%20%20
      (Variables|/Script/VRacer.VehiclePawn|SetCheckpointTransform _asvehicle_pawn_bp (Transformation|GetWorldTransform (Variables|/Script/VRacer.VehiclePawn|GetVehicleComponent _asvehicle_pawn_bp)))
      (Default|ShowCheckpointTime _asvehicle_pawn_bp)
      (Variables|/Script/VRacer.VehiclePawn|SetRaceTime _asvehicle_pawn_bp 0.0)
      (Variables|/Script/VRacer.VehiclePawn|SetbCanCount _asvehicle_pawn_bp true))))

(event Custom|StartLights
  ;[1 1 1] Play Light Cycle Sequence and Enable Vehicle
  (Rendering|Material|SetVectorParameterValue :self (Variables|Default|GetYellowLightMI) :ParameterName "Emissive" :!class /Script/Engine.MaterialInstanceDynamic)
  (Rendering|Material|SetVectorParameterValue (Variables|Default|GetRedLightMI) "Emissive" "(R=15.000000,G=0.000000,B=0.000000,A=1.000000)" :!class /Script/Engine.MaterialInstanceDynamic)
  (Utilities|FlowControl|Delay 1.0)
  (Rendering|Material|SetVectorParameterValue :self (Variables|Default|GetRedLightMI) :ParameterName "Emissive" :!class /Script/Engine.MaterialInstanceDynamic)
  (Rendering|Material|SetVectorParameterValue (Variables|Default|GetYellowLightMI) "Emissive" "(R=15.000000,G=15.000000,B=0.000000,A=1.000000)" :!class /Script/Engine.MaterialInstanceDynamic)
  (Utilities|FlowControl|Delay 1.0)
  (Rendering|Material|SetVectorParameterValue (Variables|Default|GetYellowLightMI) "Emissive" "(R=0.000000,G=0.000000,B=0.000000,A=1.000000)" :!class /Script/Engine.MaterialInstanceDynamic)
  (Rendering|Material|SetVectorParameterValue (Variables|Default|GetGreenLightMI) "Emissive" "(R=0.000000,G=15.000000,B=0.000000,A=1.000000)" :!class /Script/Engine.MaterialInstanceDynamic)
  (CallFunction|EnableVehicles))

(event EventBeginPlay
  ;[1 1 1] Start Race with Delay
  (Utilities|FlowControl|Delay 5.0)
  (CallFunction|StartLights))

(fn ConstructionScript
  (bind _returnvalue (Rendering|Material|CreateDynamicMaterialInstance (Variables|Default|GetRoadComponent) 8 "/Game/Materials/RedLightMI.RedLightMI" "None" :!class /Script/Engine.PrimitiveComponent))
  (Variables|Default|SetRedLightMI _returnvalue)
  (bind _returnvalue_2 (Rendering|Material|CreateDynamicMaterialInstance (Variables|Default|GetRoadComponent) 9 "/Game/Materials/YellowLightMI.YellowLightMI" "None" :!class /Script/Engine.PrimitiveComponent))
  (Variables|Default|SetYellowLightMI _returnvalue_2)
  (bind _returnvalue_3 (Rendering|Material|CreateDynamicMaterialInstance (Variables|Default|GetRoadComponent) 10 "/Game/Materials/GreenLightMI.GreenLightMI" "None" :!class /Script/Engine.PrimitiveComponent))
  (Variables|Default|SetGreenLightMI _returnvalue_3)
  (Rendering|Material|SetVectorParameterValue :self (Variables|Default|GetYellowLightMI) :ParameterName "Emissive" :!class /Script/Engine.MaterialInstanceDynamic))

(fn EnableVehicles
  ;[1 1 1] Enable Driving in All Vehicles
  (bind _outactors (Actor|GetAllActorsOfClass "/Game/Blueprints/VehiclePawn_BP.VehiclePawn_BP_C"))
  (for _array_element _outactors
    (Variables|/Script/VRacer.VehiclePawn|SetbCanDrive _array_element true)))